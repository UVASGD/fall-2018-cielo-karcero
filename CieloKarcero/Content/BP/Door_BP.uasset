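; Interactable door Blueprint that toggles open and closed and can be locked by the state of other interactables.
; NewInteract plays or reverses a timeline by ToggleVal over MoveTime, scaling translation and rotation offsets onto Object.
; During movement, IntArea is pinned to the world transform cached at BeginPlay.
; Tick sets Locked through CheckConflicts, which tests ToggleVal across the lock-when-open and lock-when-closed lists.
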(event EventBeginPlay
  (|CallParentFunction)
  (Variables|Default|SetIntTrans (Transformation|GetWorldTransform (Variables|Default|GetIntArea))))

(event Collision|EventActorBeginOverlap
  (params (OtherActor :type Actor%20Object%20Reference))
  (|CallParentFunction OtherActor) ; This node is disabled and will not be called.\nDrag off pins to build functionality.
)

(event EventTick
  (params (DeltaSeconds :type Float%20%28single-precision%29))
  (|CallParentFunction DeltaSeconds)
  (bind _newlock (CallFunction|CheckConflicts))
  (Variables|Default|SetLocked _newlock))

(event EventNewInteract
  (bind _object (Variables|Default|GetObject))
  (bind _inttrans (Variables|Default|GetIntTrans))
  (Utilities|FlowControl|Sequence
    (:then_0
      (Components|Timeline|SetPlayRate (Variables|Default|GetBlendOpenClose) (/ 1.0 (Variables|Default|GetMoveTime)))
      (if (Variables|Default|GetToggleVal)
        (bind _blend (Timeline|BlendOpenClose Play)
          (:Update
            (Transformation|SetRelativeLocation _object (* (Variables|Default|GetTrans) _blend) false false)
            (Transformation|SetRelativeRotation _object (* (Variables|Default|GetRot) _blend) false false)
            (Transformation|SetWorldLocationAndRotation (Variables|Default|GetIntArea) (.location _inttrans) (.rotation _inttrans) false false)))
        (else
          (Timeline|BlendOpenClose Reverse))))))

(fn ConstructionScript
  (|CallParentFunction))

(fn CheckConflicts
  (bind _lockoninteractableclosed (Variables|Default|GetLockOnInteractableClosed))
  (bind _lockoninteractableopen (Variables|Default|GetLockOnInteractableOpen))
  (Utilities|FlowControl|Sequence
    (:then_0
      (LocalVariables|SetTempLock false)
      (if (> (Utilities|Array|Length _lockoninteractableopen) 0)
        (for _array_element _lockoninteractableopen
          (if (Variables|/Game/BP/Interactible_BP.Interactible_BP_C|GetToggleVal _array_element)
            (LocalVariables|SetTempLock true)))))
    (:then_1
      (if (> (Utilities|Array|Length _lockoninteractableclosed) 0)
        (for _array_element_2 _lockoninteractableclosed
          (if (not (Variables|/Game/BP/Interactible_BP.Interactible_BP_C|GetToggleVal _array_element_2))
            (LocalVariables|SetTempLock true)))))
    (:then_2
      (return (LocalVariables|GetTempLock)))))
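; Holdable physics object that the first-person character can pick up through interaction.
; The construction script enables physics simulation on the Object component.
; On NewInteract, it casts the interacting player's pawn to FP_Char_Test_BP, rescales Object to HoldingScale, then calls the character's PHGrab to perform the grab.
; The grab logic lives in the character, and nothing here restores the original scale.
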(event EventBeginPlay
  (|CallParentFunction) ; This node is disabled and will not be called.\nDrag off pins to build functionality.
)

(event Collision|EventActorBeginOverlap
  (params (OtherActor :type Actor%20Object%20Reference))
  (|CallParentFunction OtherActor) ; This node is disabled and will not be called.\nDrag off pins to build functionality.
)

(event EventTick
  (params (DeltaSeconds :type Float%20%28single-precision%29))
  (|CallParentFunction DeltaSeconds) ; This node is disabled and will not be called.\nDrag off pins to build functionality.
)

(event EventNewInteract
  (params (Player :type Integer))
  (bind _asfp_char_test_bp (Utilities|Casting|CastToFP_Char_Test_BP (Game|Player|GetPlayerPawn Player)))
  (Transformation|SetRelativeScale3D (Variables|Default|GetObject) (Variables|Default|GetHoldingScale))
  (Default|PHGrab _asfp_char_test_bp))

(fn ConstructionScript
  (|CallParentFunction)
  (Physics|SetSimulatePhysics (Variables|Default|GetObject) true))
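; Health crystal Blueprint, a usable child actor that restores health to the player when used.
; Its ChildrenUsed event takes a Player input, fetches that player's pawn and casts it to FP_Char_Test_BP.
; It then adds a fixed amount to the character's Health, clamped to a fixed range.
; BeginPlay, overlap and Tick are disabled stubs, and the construction script only calls the parent.
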(event EventBeginPlay
  (|CallParentFunction) ; This node is disabled and will not be called.\nDrag off pins to build functionality.
)

(event Collision|EventActorBeginOverlap
  (params (OtherActor :type Actor%20Object%20Reference))
  (|CallParentFunction OtherActor) ; This node is disabled and will not be called.\nDrag off pins to build functionality.
)

(event EventTick
  (params (DeltaSeconds :type Float%20%28single-precision%29))
  (|CallParentFunction DeltaSeconds) ; This node is disabled and will not be called.\nDrag off pins to build functionality.
)

(event EventChildrenUsed
  (params (Index :type Integer) (Player :type Integer))
  (bind _asfp_char_test_bp (Utilities|Casting|CastToFP_Char_Test_BP (Game|Player|GetPlayerPawn Player)))
  (Variables|/Game/FirstPersonBP/Blueprints/FP_Char_Test_BP.FP_Char_Test_BP_C|SetHealth _asfp_char_test_bp (Math|Float|Clamp(Float) (+ (Variables|/Game/FirstPersonBP/Blueprints/FP_Char_Test_BP.FP_Char_Test_BP_C|GetHealth _asfp_char_test_bp) 5e+02) 0.0 1e+03)))

(fn ConstructionScript
  (|CallParentFunction))
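; Assault rocket rifle weapon Blueprint that fires a projectile when used.
; UseWeapon waits briefly, plays the use sound at a mesh socket, then spawns Projectile_BP.
; The projectile starts at the bullet socket but takes its rotation from the player's first-person camera, so it follows the view rather than the barrel.
; A disconnected hitscan branch with line trace, explosion effect and direct damage remains in the graph but never runs.
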(event EventBeginPlay
  (|CallParentFunction) ; This node is disabled and will not be called.\nDrag off pins to build functionality.
)

(event Collision|EventActorBeginOverlap
  (params (OtherActor :type Actor%20Object%20Reference))
  (|CallParentFunction OtherActor) ; This node is disabled and will not be called.\nDrag off pins to build functionality.
)

(event EventTick
  (params (DeltaSeconds :type Float%20%28single-precision%29))
  (|CallParentFunction DeltaSeconds) ; This node is disabled and will not be called.\nDrag off pins to build functionality.
)

(event EventUseWeapon
  (bind _skeletalmesh (Variables|Default|GetSkeletalMesh))
  (bind _bulletsocket (Variables|Default|GetBulletSocket))
  (bind _returnvalue (Transformation|GetSocketTransform _skeletalmesh _bulletsocket "RTS_World"))
  (Utilities|FlowControl|Delay 0.2)
  (Audio|PlaySoundatLocation (Variables|Default|GetUseSound) (Transformation|GetSocketLocation (Variables|Default|GetSkeletalMesh) (Variables|Default|GetSoundSocket)))
  (Game|SpawnActorfromClass "/Game/BP/Projectile_BP.Projectile_BP_C" (Math|Transform|MakeTransform (.location _returnvalue) (.rotation (Transformation|GetWorldTransform (Variables|/Game/FirstPersonBP/Blueprints/FP_Char_Test_BP.FP_Char_Test_BP_C|GetFirstPersonCamera (Variables|Default|GetPlayerRef)))) (.scale _returnvalue)) "Undefined" 0 0))

(fn ConstructionScript
  (|CallParentFunction))
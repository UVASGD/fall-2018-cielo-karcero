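; Base Blueprint for interactible objects, with an empty NewInteract event for child Blueprints to implement.
; The IntArea overlap registers and unregisters the object with FP_Char_Test_BP characters.
; Interaction2 flips the RepNotify ToggleVal and fires NewInteract unless Locked.
; The construction script applies mesh and scale overrides, while SetHighlight toggles custom depth with a stencil value that distinguishes locked objects.
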(event OnComponentBeginOverlap(IntArea)
  (params (OverlappedComponent :type Primitive%20Component%20Object%20Reference) (OtherActor :type Actor%20Object%20Reference) (OtherComp :type Primitive%20Component%20Object%20Reference) (OtherBodyIndex :type Integer) (bFromSweep :type Boolean) (SweepResult :type Hit%20Result%20Structure%20%28by%20ref%29))
  ;[1 1 1] Register Interactible On Overlap
  (bind _asfp_char_test_bp (Utilities|Casting|CastToFP_Char_Test_BP OtherActor))
  (Class|BPIInteract|RegInt(Message) _asfp_char_test_bp self))

(event OnComponentEndOverlap(IntArea)
  (params (OverlappedComponent :type Primitive%20Component%20Object%20Reference) (OtherActor :type Actor%20Object%20Reference) (OtherComp :type Primitive%20Component%20Object%20Reference) (OtherBodyIndex :type Integer))
  ;[1 1 1] Unregister Interactible On End Overlap
  (bind _asfp_char_test_bp (Utilities|Casting|CastToFP_Char_Test_BP OtherActor))
  (Class|BPIInteract|UnregInt(Message) _asfp_char_test_bp self))

(event Custom|Interaction2
  (params (Player :type Integer))
  ;[1 1 1] Interact Called - Check if Object Locked - Call Interact Functions on Child Blueprints
  (if (not (Variables|Default|GetLocked))
    (Variables|Default|SetToggleVal (not (Variables|Default|GetToggleVal)))
    (CallFunction|NewInteract Player)))

(event Custom|NewInteract
  (params (Player :type Integer)))

(event EventBeginPlay)

(event Collision|EventActorBeginOverlap
  (params (OtherActor :type Actor%20Object%20Reference)))

(event EventTick
  (params (DeltaSeconds :type Float%20%28single-precision%29)))

(fn ConstructionScript
  (bind _objectmesh (Variables|Default|GetObjectMesh))
  ;[1 1 1] Override Mesh & Mesh Scale
  (Transformation|SetRelativeScale3D (Variables|Default|GetObject) (Variables|Default|GetMeshScale))
  (if (!= _objectmesh 0)
    (Components|StaticMesh|SetStaticMesh (Variables|Default|GetObject) _objectmesh)))

(fn OnRepToggleVal)

(fn SetHighlight
  (params (UseHL :type Boolean))
  (bind _object (Variables|Default|GetObject))
  ;[1 1 1] Highlight Object
  (Rendering|SetRenderCustomDepth _object UseHL)
  (Rendering|SetCustomDepthStencilValue _object (select (Variables|Default|GetLocked) 2 5)))
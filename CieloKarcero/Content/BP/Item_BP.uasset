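; Item actor for the inventory system that handles being used, discarded or read, based on its category.
; Discarding calls UseItemTemp on the player and removes one from the inventory slot, while using removes one only for Consumables.
; Using a Readable disables the inventory widget and opens a note widget on the main canvas with UI-only input.
; The read event closes the note, re-enables the inventory and restores game-and-UI input.
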(event Custom|EventOnUsed
  (params (Index :type Integer))
  (bind _inventory (Variables|Default|GetInventory))
  (bind _mainwidget (Variables|/Game/BP/Inventory_BP.Inventory_BP_C|GetMainWidget _inventory))
  (if (Utilities|Select :Index (.Category (Utilities|Struct|BreakItem_Info_Struct (Variables|Default|GetItemInfo))) :NewEnumerator0 true :NewEnumerator1 false :NewEnumerator2 false :NewEnumerator3 false)
    (Default|RemoveItematIndex (Variables|Default|GetInventory) (Variables|Default|GetIndex) 1))
  (if (Utilities|Enum|Equal(Enum) (.Category (Utilities|Struct|BreakItem_Info_Struct (Variables|Default|GetItemInfo))) "NewEnumerator1")
    (Widget|SetIsEnabled (Variables|/Game/UI/Inventory/Widgets/Main_Inventory_Widget.Main_Inventory_Widget_C|GetInventory_Widget _mainwidget) false)
    (bind _returnvalue (UserInterface|CreateWidget "/Game/UI/Inventory/Widgets/Note_Widget.Note_Widget_C" 0 self))
    (bind _output_get (Variables|Default|SetNoteWidget _returnvalue))
    (bind _returnvalue_2 (Class|CanvasPanel|AddChildtoCanvas (Variables|/Game/UI/Inventory/Widgets/Main_Inventory_Widget.Main_Inventory_Widget_C|GetMainCanvas _mainwidget) _output_get))
    (Class|CanvasPanelSlot|SetAnchors _returnvalue_2 (Utilities|Struct|MakeAnchors "(X=0.500000,Y=0.000000)" "(X=0.500000,Y=1.000000)"))
    (Class|CanvasPanelSlot|SetAutoSize _returnvalue_2 true)
    (Class|CanvasPanelSlot|SetPosition _returnvalue_2 (Math|Vector2D|MakeVector2D -4.5e+02 0.0))
    (Input|SetInputModeUIOnly (Game|GetPlayerController 0) (Variables|Default|GetNoteWidget) "DoNotLock")))

(event Custom|EventOnRead
  (if (Utilities|Enum|Equal(Enum) (.Category (Utilities|Struct|BreakItem_Info_Struct (Variables|Default|GetItemInfo))) "NewEnumerator1")
    (Widget|SetIsEnabled (Variables|/Game/UI/Inventory/Widgets/Main_Inventory_Widget.Main_Inventory_Widget_C|GetInventory_Widget (Variables|/Game/BP/Inventory_BP.Inventory_BP_C|GetMainWidget (Variables|Default|GetInventory))) true)
    (Widget|RemovefromParent (Variables|Default|GetNoteWidget))
    (Input|SetInputModeGameandUI (Game|GetPlayerController 0) 0 "DoNotLock" false)))

(event Custom|EventOnDiscarded
  (params (Index :type Integer))
  (Default|UseItemTemp (Variables|/Game/BP/Inventory_BP.Inventory_BP_C|GetPlayerRef (Variables|Default|GetInventory)) Index)
  (Default|RemoveItematIndex (Variables|Default|GetInventory) (Variables|Default|GetIndex) 1))

(event EventBeginPlay
  (|CallParentFunction) ; This node is disabled and will not be called.\nDrag off pins to build functionality.
)

(event Collision|EventActorBeginOverlap
  (params (OtherActor :type Actor%20Object%20Reference))
  (|CallParentFunction OtherActor) ; This node is disabled and will not be called.\nDrag off pins to build functionality.
)

(event EventTick
  (params (DeltaSeconds :type Float%20%28single-precision%29))
  (|CallParentFunction DeltaSeconds) ; This node is disabled and will not be called.\nDrag off pins to build functionality.
)

(fn ConstructionScript
  (|CallParentFunction))
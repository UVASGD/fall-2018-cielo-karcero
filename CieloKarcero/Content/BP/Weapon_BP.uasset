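; Weapon item Blueprint that equips itself on the player when used.
; Its onUsed event calls EquipItem on the player reference held by its Inventory, passing itself with Load set to false.
; The other events are disabled stubs and the construction script only calls the parent, so the equip logic lives in the player.
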(event EventBeginPlay
  (|CallParentFunction) ; This node is disabled and will not be called.\nDrag off pins to build functionality.
)

(event Collision|EventActorBeginOverlap
  (params (OtherActor :type Actor%20Object%20Reference))
  (|CallParentFunction OtherActor) ; This node is disabled and will not be called.\nDrag off pins to build functionality.
)

(event EventTick
  (params (DeltaSeconds :type Float%20%28single-precision%29))
  (|CallParentFunction DeltaSeconds) ; This node is disabled and will not be called.\nDrag off pins to build functionality.
)

(event EventEventonUsed
  (params (Index :type Integer) (Player :type Integer))
  (Default|EquipItem (Variables|/Game/BP/Inventory_BP.Inventory_BP_C|GetPlayerRef (Variables|Default|GetInventory)) self false))

(fn ConstructionScript
  (|CallParentFunction))
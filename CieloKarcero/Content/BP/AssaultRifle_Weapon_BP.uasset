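; Assault rifle weapon Blueprint that fires a hitscan shot when its UseWeapon event runs.
; After a short delay, it plays the use sound at the mesh's sound socket and line traces on the Visibility channel from the player's first-person camera, ignoring the player.
; A hit spawns an explosion emitter at the impact and applies fixed damage to the hit actor.
; The bullet socket nodes are unused.
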(event EventBeginPlay
  (|CallParentFunction) ; This node is disabled and will not be called.\nDrag off pins to build functionality.
)

(event Collision|EventActorBeginOverlap
  (params (OtherActor :type Actor%20Object%20Reference))
  (|CallParentFunction OtherActor) ; This node is disabled and will not be called.\nDrag off pins to build functionality.
)

(event EventTick
  (params (DeltaSeconds :type Float%20%28single-precision%29))
  (|CallParentFunction DeltaSeconds) ; This node is disabled and will not be called.\nDrag off pins to build functionality.
)

(event EventUseWeapon
  (bind _playerref (Variables|Default|GetPlayerRef))
  (bind _firstpersoncamera (Variables|/Game/FirstPersonBP/Blueprints/FP_Char_Test_BP.FP_Char_Test_BP_C|GetFirstPersonCamera _playerref))
  (bind _returnvalue (Transformation|GetWorldLocation _firstpersoncamera))
  (Utilities|FlowControl|Delay 0.2)
  (Audio|PlaySoundatLocation (Variables|Default|GetUseSound) (Transformation|GetSocketLocation (Variables|Default|GetSkeletalMesh) (Variables|Default|GetSoundSocket)))
  (bind (_outhit _returnvalue_2) (Collision|LineTraceByChannel _returnvalue (+ _returnvalue (* (Math|Vector|GetForwardVector _firstpersoncamera) 1e+04)) "TraceTypeQuery1" false (Utilities|Array|MakeArray _playerref) "None"))
  (if _returnvalue_2
    (Effects|SpawnEmitteratLocation "/Game/StarterContent/Particles/P_Explosion.P_Explosion" (.Location (Collision|BreakHitResult _outhit)))
    (Game|Damage|ApplyDamage (.HitActor (Collision|BreakHitResult _outhit)) 3e+02 0 0)))

(fn ConstructionScript
  (|CallParentFunction))
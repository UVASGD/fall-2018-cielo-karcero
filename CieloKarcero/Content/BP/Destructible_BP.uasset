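; Grabbable physics prop that shatters by swapping its Object component for a Destructible one when hit hard enough.
; Interacting calls PHGrab on the player's FP_Char_Test_BP pawn.
; Construction scales the Destructible and, if a mesh override is set, applies it and keeps it hidden and inert.
; An impact above Fragility activates the Destructible and disables Object; the node aligning their transforms is disconnected.
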(event OnComponentHit(Object)
  (params (HitComponent :type Primitive%20Component%20Object%20Reference) (OtherActor :type Actor%20Object%20Reference) (OtherComp :type Primitive%20Component%20Object%20Reference) (NormalImpulse :type Vector :default "0, 0, 0") (Hit :type Hit%20Result%20Structure%20%28by%20ref%29))
  (bind _object (Variables|Default|GetObject))
  (bind _destructible (Variables|Default|GetDestructible))
  (if (> (Math|Vector|VectorLength NormalImpulse) (Variables|Default|GetFragility))
    (Development|SetHiddeninGame _destructible false false)
    (Collision|SetCollisionEnabled _destructible "QueryAndPhysics")
    (Components|Tick|SetComponentTickEnabled _destructible true)
    (Physics|SetSimulatePhysics _destructible true)
    (Physics|SetSimulatePhysics _object false)
    (Development|SetHiddeninGame _object true false)
    (Collision|SetCollisionEnabled _object "NoCollision")
    (Components|Tick|SetComponentTickEnabled _object false)))

(event EventBeginPlay
  (|CallParentFunction))

(event Collision|EventActorBeginOverlap
  (params (OtherActor :type Actor%20Object%20Reference))
  (|CallParentFunction OtherActor) ; This node is disabled and will not be called.\nDrag off pins to build functionality.
)

(event EventTick
  (params (DeltaSeconds :type Float%20%28single-precision%29))
  (|CallParentFunction DeltaSeconds))

(event EventNewInteract
  (bind _asfp_char_test_bp (Utilities|Casting|CastToFP_Char_Test_BP (Game|Player|GetPlayerPawn 0)))
  (Default|PHGrab _asfp_char_test_bp))

(fn ConstructionScript
  (bind _destructible (Variables|Default|GetDestructible))
  (|CallParentFunction)
  ;[1 1 1] Override Mesh
  (Transformation|SetRelativeScale3D (Variables|Default|GetDestructible) (Variables|Default|GetDM_Scale))
  (if (!= (Variables|Default|GetDestructibleMesh) 0)
    (Class|DestructibleComponent|SetDestructibleMesh (Variables|Default|GetDestructible) (Variables|Default|GetDestructibleMesh))
    (Physics|SetSimulatePhysics _destructible false)
    (Development|SetHiddeninGame _destructible true false)
    (Collision|SetCollisionEnabled _destructible "NoCollision")
    (Components|Tick|SetComponentTickEnabled _destructible false)))
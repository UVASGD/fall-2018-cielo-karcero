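; Speed boost actor that temporarily changes the first-person test character's walk speed when used.
; On ChildrenUsed it gets that player's pawn as FP_Char_Test_BP, saves its MaxWalkSpeed and applies NewSpeed.
; After a BoostDelay wait it restores the saved speed, printing debug messages at the start and end.
; BeginPlay, overlap and Tick are disabled stubs, so all behavior runs from that one event.
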(event EventBeginPlay
  (|CallParentFunction) ; This node is disabled and will not be called.\nDrag off pins to build functionality.
)

(event Collision|EventActorBeginOverlap
  (params (OtherActor :type Actor%20Object%20Reference))
  (|CallParentFunction OtherActor) ; This node is disabled and will not be called.\nDrag off pins to build functionality.
)

(event EventTick
  (params (DeltaSeconds :type Float%20%28single-precision%29))
  (|CallParentFunction DeltaSeconds) ; This node is disabled and will not be called.\nDrag off pins to build functionality.
)

(event EventChildrenUsed
  (params (Index :type Integer) (Player :type Integer))
  (bind _asfp_char_test_bp (Utilities|Casting|CastToFP_Char_Test_BP (Game|Player|GetPlayerPawn Player)))
  (Development|PrintString "Speeeed")
  (Variables|Default|SetOldSpeed (Variables|/Script/Engine.CharacterMovementComponent|GetMaxWalkSpeed (Variables|/Script/Engine.Character|GetCharacterMovement _asfp_char_test_bp)))
  (Variables|/Script/Engine.CharacterMovementComponent|SetMaxWalkSpeed (Variables|/Script/Engine.Character|GetCharacterMovement _asfp_char_test_bp) (Variables|Default|GetNewSpeed))
  (Utilities|FlowControl|Delay (Variables|Default|GetBoostDelay))
  (Development|PrintString "No speeeed")
  (Variables|/Script/Engine.CharacterMovementComponent|SetMaxWalkSpeed (Variables|/Script/Engine.Character|GetCharacterMovement _asfp_char_test_bp) (Variables|Default|GetOldSpeed)))

(fn ConstructionScript
  (|CallParentFunction))
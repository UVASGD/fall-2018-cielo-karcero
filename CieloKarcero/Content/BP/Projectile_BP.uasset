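; Projectile actor that launches its mesh forward with a physics impulse on BeginPlay and explodes on hit.
; On hit it spawns fire particles and a sound, runs a 1000-unit sphere overlap, then destroys itself.
; Each overlapped actor yields clamped inverse-distance damage, but the ApplyDamage call shows no damaged actor wired.
; Debug strings print on impact and when the overlap finds actors.
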(event OnComponentHit(StaticMesh)
  (params (HitComponent :type Primitive%20Component%20Object%20Reference) (OtherActor :type Actor%20Object%20Reference) (OtherComp :type Primitive%20Component%20Object%20Reference) (NormalImpulse :type Vector :default "0, 0, 0") (Hit :type Hit%20Result%20Structure%20%28by%20ref%29))
  (bind _location (Collision|BreakHitResult Hit))
  (bind _staticmesh (Variables|Default|GetStaticMesh))
  (bind _returnvalue (Transformation|GetWorldLocation _staticmesh))
  (Development|PrintString "Boom")
  (Effects|SpawnEmitteratLocation "/Game/StarterContent/Particles/P_Fire.P_Fire" _location)
  (Audio|SpawnSoundatLocation "/Engine/VREditor/Sounds/UI/Click_on_Button_Cue.Click_on_Button_Cue" _location)
  (bind (_outactors _returnvalue_2) (Collision|SphereOverlapActors _returnvalue 1e+03 (Utilities|Array|MakeArray "ObjectTypeQuery1" "ObjectTypeQuery2" "ObjectTypeQuery3" "ObjectTypeQuery4") 0))
  (if _returnvalue_2
    (Development|PrintString "Hello")
    (for _array_element _outactors
      (Game|Damage|ApplyDamage 0 (Math|Float|Clamp(Float) (/ 3e+02 (Math|Vector|VectorLength (- (Transformation|GetActorLocation _array_element) _returnvalue))) 0.0 3e+02) 0 0)))
  (Actor|DestroyActor))

(event EventBeginPlay
  (bind _staticmesh (Variables|Default|GetStaticMesh))
  (Physics|AddImpulse _staticmesh (* (Math|Vector|GetForwardVector _staticmesh) 1e+05) "None" false))

(event Collision|EventActorBeginOverlap
  (params (OtherActor :type Actor%20Object%20Reference)))

(event EventTick
  (params (DeltaSeconds :type Float%20%28single-precision%29)))

(fn ConstructionScript)
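; Light_BP is an interactable light actor whose visibility follows the ToggleVal boolean.
; The construction script applies the initial state, and the NewInteract event reapplies it using whatever value ToggleVal holds, without flipping it here.
; When UseLightMat is set, both also choose between two materials for the named LightMatSlot on Object to match the on/off state.
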(event EventBeginPlay
  (|CallParentFunction) ; This node is disabled and will not be called.\nDrag off pins to build functionality.
)

(event Collision|EventActorBeginOverlap
  (params (OtherActor :type Actor%20Object%20Reference))
  (|CallParentFunction OtherActor) ; This node is disabled and will not be called.\nDrag off pins to build functionality.
)

(event EventTick
  (params (DeltaSeconds :type Float%20%28single-precision%29))
  (|CallParentFunction DeltaSeconds) ; This node is disabled and will not be called.\nDrag off pins to build functionality.
)

(event EventNewInteract
  (params (Player :type Integer))
  ;[1 1 1] Toggle Light & Light Material - Need to create ON/OFF light materials
  (Rendering|SetVisibility (Variables|/Script/Engine.Light|GetLightComponent (Variables|Default|GetLightComp)) (Variables|Default|GetToggleVal) false)
  (if (Variables|Default|GetUseLightMat)
    (Rendering|Material|SetMaterialbyName (Variables|Default|GetObject) (Variables|Default|GetLightMatSlot) (select (Variables|Default|GetToggleVal) 0 0))))

(fn ConstructionScript
  (|CallParentFunction)
  ;[1 1 1] Initialize Light & Light Materials - Need to create basic ON/OFF light materials
  (Rendering|SetVisibility (Variables|/Script/Engine.Light|GetLightComponent (Variables|Default|GetLightComp)) (Variables|Default|GetToggleVal) false)
  (if (Variables|Default|GetUseLightMat)
    (Rendering|Material|SetMaterialbyName (Variables|Default|GetObject) (Variables|Default|GetLightMatSlot) (select (Variables|Default|GetToggleVal) 0 0))))
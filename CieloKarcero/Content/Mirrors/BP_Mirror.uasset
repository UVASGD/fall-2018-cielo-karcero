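; Mirror actor, derived from a scene capture parent, that renders a planar reflection of the player camera's view through a SceneCaptureComponent2D.
; When rendering is enabled, it ticks after the camera manager and captures manually only when an update check passes.
; Before each capture it sets the clip plane to the mirror's surface and reflects the camera's location and rotation across the actor's forward-vector plane.
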(event EventBeginPlay
  (if (Variables|Default|GetbRenderEnabled)
    (CallFunction|EnableRender)
    (Actor|Tick|AddTickPrerequisiteActor (Game|GetPlayerCameraManager 0))))

(event EventUpdateSCC2DTransform
  (|CallParentFunction)
  (CallFunction|UpdateSCC2DTransformOverriden))

(event EventTick
  (params (DeltaSeconds :type Float%20%28single-precision%29))
  (if (Variables|Default|GetbRenderEnabled)
    (bind _sccneedstoupdate (CallFunction|CheckSCCNeedstoUpdate))
    (if _sccneedstoupdate
      (CallFunction|UpdateSCC2DTransform)
      (Rendering|SceneCapture|CaptureScene (Variables|Default|GetSceneCaptureComponent2D) :!class /Script/Engine.SceneCaptureComponent2D))))

(fn ConstructionScript
  (|CallParentFunction))

(fn UpdateSCC2DTransformOverriden
  (bind _returnvalue (Game|GetPlayerCameraManager 0))
  (bind _returnvalue_2 (Transformation|GetActorTransform))
  (bind _returnvalue_3 (Transformation|GetActorForwardVector))
  (bind _scenecapturecomponent2d (Variables|Default|GetSceneCaptureComponent2D))
  (bind (_location _rotation _scale) (Math|Transform|BreakTransform _returnvalue_2))
  (bind _transformcomponent (Variables|/Script/Engine.PlayerCameraManager|GetTransformComponent _returnvalue))
  (bind _returnvalue_4 (Transformation|GetWorldTransform _transformcomponent))
  (bind (_x _y _z) (Math|Rotator|GetAxes (.rotation _returnvalue_4)))
  (Variables|/Script/Engine.SceneCaptureComponent2D|SetClipPlaneBase _scenecapturecomponent2d (Transformation|GetActorLocation))
  (Variables|/Script/Engine.SceneCaptureComponent2D|SetClipPlaneNormal _scenecapturecomponent2d (Transformation|GetActorForwardVector))
  (LocalVariables|Setlocal_SceneCaptureLocation (Math|Transform|TransformLocation (Math|Transform|MakeTransform _location _rotation (Math|Vector|MakeVector (* (.x _scale) -1.0) (.y _scale) (.z _scale))) (Math|Transform|InverseTransformLocation _returnvalue_2 (.location _returnvalue_4))))
  (LocalVariables|Setlocal_SceneCaptureRotation (Math|Rotator|MakeRotfromXY (Math|Vector|MirrorVectorbyNormal _x _returnvalue_3) (Math|Vector|MirrorVectorbyNormal _y _returnvalue_3)))
  (Transformation|SetWorldLocationAndRotation _scenecapturecomponent2d (LocalVariables|Getlocal_SceneCaptureLocation) (LocalVariables|Getlocal_SceneCaptureRotation) false false))
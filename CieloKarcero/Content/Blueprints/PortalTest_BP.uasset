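; Test portal actor that teleports any overlapping actor to its linked OtherPortal, shifting it by the offset between the two portal roots.
; Both portals disable teleporting for a short delay to prevent immediate bouncing back.
; Helper functions map location, direction and rotation between portal transforms using mirroring but are not called here; PortalVelocity is empty.
; Render-target portal view and camera-follow logic are disconnected, so they never run.
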(event EventBeginPlay)

(event Collision|EventActorBeginOverlap
  (params (OtherActor :type Actor%20Object%20Reference))
  (if (Variables|Default|GetCanTeleport)
    (Variables|Default|SetCanTeleport false)
    (Variables|PortalTest_BP_C|SetCanTeleport (Variables|Default|GetOtherPortal) false)
    (Transformation|SetActorLocation OtherActor (+ (- (Transformation|GetWorldLocation (Variables|PortalTest_BP_C|GetDefaultSceneRoot (Variables|Default|GetOtherPortal))) (Transformation|GetWorldLocation (Variables|Default|GetDefaultSceneRoot))) (Transformation|GetActorLocation OtherActor)) false true)
    (Utilities|FlowControl|Delay 0.5)
    (Variables|Default|SetCanTeleport true)
    (Variables|PortalTest_BP_C|SetCanTeleport (Variables|Default|GetOtherPortal) true)))

(event EventTick
  (params (DeltaSeconds :type Float%20%28single-precision%29)))

(fn ConstructionScript)

(fn PortalDirection
  (params (TargetPortal :type Portal%20Test%20BP%20Object%20Reference) (PrevDir :type Vector))
  (return (Math|Transform|TransformDirection (Transformation|GetActorTransform TargetPortal) (Math|Vector|MirrorVectorbyNormal (Math|Vector|MirrorVectorbyNormal (Math|Transform|InverseTransformDirection (Transformation|GetActorTransform) PrevDir) "1.000000, 0, 0") "0,1.000000, 0"))))

(fn PortalLocation
  (params (TargetPortal :type Portal%20Test%20BP%20Object%20Reference) (PrevLoc :type Vector))
  (bind _returnvalue (Transformation|GetActorTransform))
  (bind (_location _rotation _scale) (Math|Transform|BreakTransform _returnvalue))
  (return (Math|Transform|TransformLocation (Transformation|GetActorTransform TargetPortal) (Math|Transform|InverseTransformLocation (Math|Transform|MakeTransform _location _rotation (Math|Vector|MakeVector (* (.x _scale) -1.0) (* (.y _scale) -1.0) (.z _scale))) PrevLoc))))

(fn PortalLocationMirrored
  (params (TargetPortal :type Portal%20Test%20BP%20Object%20Reference) (PrevLoc :type Vector))
  (bind _returnvalue (Transformation|GetActorTransform))
  (bind (_location _rotation _scale) (Math|Transform|BreakTransform _returnvalue))
  (return (Math|Transform|TransformLocation (Transformation|GetActorTransform TargetPortal) (Math|Transform|InverseTransformLocation (Math|Transform|MakeTransform _location _rotation (Math|Vector|MakeVector (.x _scale) (* (.y _scale) -1.0) (.z _scale))) PrevLoc))))

(fn PortalRotation
  (params (TargetPortal :type Portal%20Test%20BP%20Object%20Reference) (PrevRot :type Rotator))
  (bind (_x _y) (Math|Rotator|GetAxes PrevRot))
  (bind _outdir (CallFunction|PortalDirection TargetPortal _x))
  (bind _outdir_2 (CallFunction|PortalDirection TargetPortal _y))
  (return (Math|Rotator|MakeRotfromXY _outdir _outdir_2)))

(fn PortalVelocity)